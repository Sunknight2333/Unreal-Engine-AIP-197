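; Player controller for a networked platformer that tracks coins, a key, the nearby door and respawning.
; Server events store state, then client events update the HUD, locked-door message and win screen.
; On unpossess it asks ThirdPersonGameMode to respawn it, and ServerRespawn spawns and possesses a new EpicCharacter after a short delay.
; Interact input has the server open the stored door, passing this controller.
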(event `Client_HUD`
  ;[0 0.9162 1] Display HUD
  (bind _returnvalue (`|CreateWidget` "/Game/Hour_of_Code/Widgets/W_HUD.W_HUD_C"))
  (bind _output_get (set `self.W_HUD_ref` _returnvalue))
  (`UserWidget.AddToViewport` _output_get 0))

(event `ServerRespawn`
  (params (`Spawn Transform Location` :type "Vector Structure") (`Spawn Transform Scale` :type "Vector Structure") (`Spawn Transform Rotation` :type "Rotator Structure"))
  (bind (_spawntransform_location _spawntransform_rotation) (`KismetMathLibrary.BreakTransform` (`self.SpawnTransform`)))
  (bind _returnvalue (`|SpawnActorFromClass` "/Game/ThirdPersonBP/Blueprints/EpicCharacter.EpicCharacter_C" (`KismetMathLibrary.MakeTransform` _spawntransform_location _spawntransform_rotation) "Undefined" "OverrideRootScale" null null))
  (`KismetSystemLibrary.Delay` 1.0)
  (`self.Possess` _returnvalue))

(event `self.ReceiveUnPossess`
  (params (UnpossessedPawn :type "Pawn Object Reference"))
  (bind _asthird_person_game_mode (cast `/Game/ThirdPersonBP/Blueprints/ThirdPersonGameMode` (`GameplayStatics.GetGameMode`)))
  (`/Game/ThirdPersonBP/Blueprints/ThirdPersonGameMode.Respawn` _asthird_person_game_mode self))

(event `Server_StoreSpawnTransform`
  (params (SpawnTransform :type "Transform Structure"))
  (set `self.SpawnTransform` SpawnTransform))

(event `Server_AddCoins`
  (params (coins :type Integer))
  (bind _output_get (set `self.coins` (+ (`self.coins`) coins)))
  (`self.Client_UpdateCoinUI` _output_get))

(event `Client_UpdateCoinUI`
  (params (CoinAmount :type Integer))
  (`/Game/Hour_of_Code/Widgets/W_HUD.updateCoins` (`self.W_HUD_ref`) CoinAmount))

(event `Server_UpdateKey`
  (params (Key :type Boolean))
  (bind _output_get (set `self.HaveKey?` Key))
  (`self.Client_UpdateKeyUI` _output_get))

(event `Client_UpdateKeyUI`
  (params (HasKey :type Boolean))
  (bind _t_key (`/Game/Hour_of_Code/Widgets/W_HUD.T_Key` (`self.W_HUD_ref`)))
  (if HasKey
    (`Image.SetColorAndOpacity` _t_key (struct :`R` 1.0 :`G` 1.0 :`B` 1.0 :`A` 1.0))
    (else
      (`Image.SetColorAndOpacity` _t_key (struct :`R` 1.0 :`G` 1.0 :`B` 1.0 :`A` 0.3)))))

(event `Server_Door`
  (params (State :type Boolean) (DoorRef :type "/Game/Hour_of_Code/Blueprints/BP_Door_Locked_activity_4_end Object Reference"))
  (if State
    (set `self.Door Ref` DoorRef)
    (else
      (set `self.Door Ref` null))))

(event `Client_ShowMessageUI`
  (params (ShowMessage :type Boolean))
  (if ShowMessage
    (bind _returnvalue (`|CreateWidget` "/Game/Hour_of_Code/Widgets/W_lockedDoor.W_lockedDoor_C"))
    (bind _output_get (set `self.MessageUI` _returnvalue))
    (`UserWidget.AddToViewport` _output_get 0)
    (else
      (bind _messageui (`self.MessageUI`)
        (:`then`
          (`Widget.RemoveFromParent` _messageui)
          (set `self.MessageUI` null))
        (:`else`)))))

(event `InputAction|Interact`
  (params (Key :type "Key Structure"))
  (:`Pressed`
    (`self.Door Ref`
      (:`then`
        (`self.Server_DoorOpen`))
      (:`else`))))

(event `Server_DoorOpen`
  (`/Game/Hour_of_Code/Blueprints/BP_Door_Locked_activity_4_end.OpenDoor` (`self.Door Ref`) self))

(event `Client_Win`
  (`self.DisableInput` self)
  (bind _returnvalue (`|CreateWidget` "/Game/Hour_of_Code/Widgets/W_gameCompletion.W_gameCompletion_C"))
  (`UserWidget.AddToViewport` _returnvalue 0)
  (`Widget.RemoveFromParent` (`self.W_HUD_ref`)))

(fn `UserConstructionScript`)